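; CardInfoUtils is a card game utility that turns an integer card ID into that card's data table row.
; MakeCardInfoFromSuitId treats IDs as blocks of eleven: below 11 reads CD_Blue, below 22 CD_Orange, anything higher CD_Red.
; The ID modulo 11 indexes the table's row-name list, so results depend on row order.
; Only the Row Found path explicitly returns a row.
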(fn `MakeCardInfoFromSuitId`
  (params (CardId :type Integer))
  (returns (OutCardInfo :type "/Game/CardGameTemplate/Blueprints/CardInfo Structure"))
  (locals (CardIndex :type Integer))
  (bind _output_get (set `local.CardIndex` CardId))
  (if (< _output_get 11)
    (bind _outrownames (`DataTableFunctionLibrary.GetDataTableRowNames` "/Game/CardGameTemplate/Blueprints/CardDatabase/CD_Blue.CD_Blue"))
    (bind _returnvalue (`|GetDataTableRow` "/Game/CardGameTemplate/Blueprints/CardDatabase/CD_Blue.CD_Blue" (`|GetArrayItem` _outrownames _output_get))
      (:`then`
        (return _returnvalue)))
    (elif (< _output_get 22)
      (bind _outrownames_2 (`DataTableFunctionLibrary.GetDataTableRowNames` "/Game/CardGameTemplate/Blueprints/CardDatabase/CD_Orange.CD_Orange"))
      (bind _returnvalue_2 (`|GetDataTableRow` "/Game/CardGameTemplate/Blueprints/CardDatabase/CD_Orange.CD_Orange" (`|GetArrayItem` _outrownames_2 (mod (`local.CardIndex`) 11)))
        (:`then`
          (return _returnvalue_2)))
      (else
        (bind _outrownames_3 (`DataTableFunctionLibrary.GetDataTableRowNames` "/Game/CardGameTemplate/Blueprints/CardDatabase/CD_Red.CD_Red"))
        (bind _returnvalue_3 (`|GetDataTableRow` "/Game/CardGameTemplate/Blueprints/CardDatabase/CD_Red.CD_Red" (`|GetArrayItem` _outrownames_3 (mod (`local.CardIndex`) 11)))
          (:`then`
            (return _returnvalue_3)))))))