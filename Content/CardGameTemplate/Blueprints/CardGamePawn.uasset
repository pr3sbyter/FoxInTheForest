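; CardGamePawn is a card game player pawn that, on BeginPlay with over six cards in the deck, spawns an attached Hand and draws thirteen cards.
; The game state's Deal flag makes the first pawn the Dealer and hides later pawns' cards.
; The dealer places a random card in the "Joker"-tagged slot, separately picks a random TrumpCard for the game state, then draws a replacement.
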(event `self.ReceiveBeginPlay`
  (bind _returnvalue (`GameplayStatics.GetGameState`))
  (bind _hand (`self.Hand`))
  (bind _output (`|GetArrayItem` (`/Game/CardGameTemplate/Blueprints/Hand.HandCards` _hand) (`KismetMathLibrary.RandomIntegerInRange` 0 12)))
  (bind _ascard_game_game_state (cast `/Game/CardGameTemplate/Blueprints/CardGameGameState` _returnvalue))
  (if (not (<= (`KismetArrayLibrary.Array_Length` (`/Game/CardGameTemplate/Blueprints/Deck.DeckCards` (`/Game/CardGameTemplate/Blueprints/CardGameGameState.Deck` _ascard_game_game_state))) 6))
    (`self.MakeHand`)
    (bind _ascard_game_game_state_2 (cast `/Game/CardGameTemplate/Blueprints/CardGameGameState` _returnvalue))
    (for _ (range 13)
      (bind _deck (`/Game/CardGameTemplate/Blueprints/CardGameGameState.Deck` _ascard_game_game_state_2))
      (`/Game/CardGameTemplate/Blueprints/Hand.DrawFromDeck` (`self.Hand`) _deck false)
      (if (`/Game/CardGameTemplate/Blueprints/CardGameGameState.Deal` _ascard_game_game_state_2)
        (for _array_element (`/Game/CardGameTemplate/Blueprints/Hand.HandCards` (`self.Hand`))
          (bind _ascard_game_game_state_3 (cast `/Game/CardGameTemplate/Blueprints/CardGameGameState` (`GameplayStatics.GetGameState`)))
          (`SceneComponent.SetHiddenInGame` (`/Game/CardGameTemplate/Blueprints/Card.Root` _array_element) (`/Game/CardGameTemplate/Blueprints/CardGameGameState.Deal` _ascard_game_game_state_3) true))))
    (bind _ascard_game_game_state_4 (cast `/Game/CardGameTemplate/Blueprints/CardGameGameState` (`GameplayStatics.GetGameState`)))
    (`|ExecutionSequence`
      (:`then_0`
        (if (not (`/Game/CardGameTemplate/Blueprints/CardGameGameState.Deal` _ascard_game_game_state_4))
          (set `/Game/CardGameTemplate/Blueprints/Hand.ClickedCard` _output _hand)
          (bind _outactors (`GameplayStatics.GetAllActorsWithTag` "Joker"))
          (bind _ascard_game_game_state_5 (cast `/Game/CardGameTemplate/Blueprints/CardGameGameState` (`GameplayStatics.GetGameState`)))
          (bind _asboard_card_slot (cast `/Game/CardGameTemplate/Blueprints/BoardCardSlot` (`|GetArrayItem` _outactors)))
          (set `/Game/CardGameTemplate/Blueprints/CardGameGameState.TrumpCard` _output _ascard_game_game_state_5)
          (`/Game/CardGameTemplate/Blueprints/Hand.PlaceCard` _hand _asboard_card_slot false)
          (set `self.Dealer` true)
          (`/Game/CardGameTemplate/Blueprints/Hand.DrawFromDeck` _hand _deck false)))
      (:`then_1`
        (set `/Game/CardGameTemplate/Blueprints/CardGameGameState.Deal` true _ascard_game_game_state_4)))))

(fn `MakeHand`
  (bind _returnvalue (`|SpawnActorFromClass` "/Game/CardGameTemplate/Blueprints/Hand.Hand_C" (`KismetMathLibrary.MakeTransform` (0.0 0.0 0.0)) "Undefined" "OverrideRootScale" null null))
  (bind _output_get (set `self.Hand` _returnvalue))
  (`self.K2_AttachToComponent` _output_get (`self.HandAttachPoint`) "None" "KeepRelative" "KeepRelative" "KeepRelative" true))

(fn `UserConstructionScript`)